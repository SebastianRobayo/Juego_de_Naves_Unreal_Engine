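; Player ship Blueprint that moves on four axis directions, fires bullets and destroys itself when its health runs out.
; Directional input actions open and close Gates that Tick feeds, adding unswept local offsets of Velocidad per frame, unscaled by delta time.
; Disparo spawns BalaDeJugador at the ship's transform.
; Tick also checks VidaJugador for death, while a BeginPlay Delay loop prints it periodically.
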(event `InputAction|Adelante`
  (params (Key :type "Key Structure"))
  ;[1 1 1] Movimiento del Jugador
  (:`Pressed`
    (goto _label_2 :!via `Open`))
  (:`Released`
    (goto _label_2 :!via `Close`)))

(event `self.ReceiveBeginPlay`
  (`KismetSystemLibrary.Delay` 2.0 :!label _label)
  (`KismetSystemLibrary.PrintString` (`KismetStringLibrary.Conv_DoubleToString` (`self.Vida_Jugador`)))
  (goto _label))

(event `InputAction|Atras`
  (params (Key :type "Key Structure"))
  ;[1 1 1] Movimiento del Jugador
  (:`Pressed`
    (goto _label_3 :!via `Open`))
  (:`Released`
    (goto _label_3 :!via `Close`)))

(event `self.ReceiveTick`
  (params (DeltaSeconds :type "Float (single-precision)"))
  (`|ExecutionSequence`
    (:`then_0`
      ;[1 1 1] Movimiento del Jugador
      (`/Engine/EditorBlueprintResources/StandardMacros.Gate` true :!label _label_2
        (:`Exit`
          (`self.K2_AddActorLocalOffset` (`KismetMathLibrary.MakeVector` (`self.Velocidad`))))))
    (:`then_1`
      (`/Engine/EditorBlueprintResources/StandardMacros.Gate` true :!label _label_3
        (:`Exit`
          (`self.K2_AddActorLocalOffset` (`KismetMathLibrary.MakeVector` (* (`self.Velocidad`) -1.0))))))
    (:`then_2`
      (`/Engine/EditorBlueprintResources/StandardMacros.Gate` true :!label _label_4
        (:`Exit`
          (`self.K2_AddActorLocalOffset` (`KismetMathLibrary.MakeVector` 0.0 (`self.Velocidad`))))))
    (:`then_3`
      (`/Engine/EditorBlueprintResources/StandardMacros.Gate` true :!label _label_5
        (:`Exit`
          (`self.K2_AddActorLocalOffset` (`KismetMathLibrary.MakeVector` 0.0 (* (`self.Velocidad`) -1.0))))))
    (:`then_4`
      ;[1 1 1] Destrucción del jugador
      (if (<= (`self.Vida_Jugador`) 0.0)
        (`self.K2_DestroyActor`)))))

(event `InputAction|Derecha`
  (params (Key :type "Key Structure"))
  ;[1 1 1] Movimiento del Jugador
  (:`Pressed`
    (goto _label_4 :!via `Open`))
  (:`Released`
    (goto _label_4 :!via `Close`)))

(event `InputAction|Izquierda`
  (params (Key :type "Key Structure"))
  ;[1 1 1] Movimiento del Jugador
  (:`Pressed`
    (goto _label_5 :!via `Open`))
  (:`Released`
    (goto _label_5 :!via `Close`)))

(event `InputAction|Disparo`
  (params (Key :type "Key Structure"))
  ;[1 1 1] Disparo Jugador
  (:`Pressed`
    (`|SpawnActorFromClass` (`self.Bala_de_Jugador`) (`self.GetTransform`) "Undefined" "OverrideRootScale" null null)))

(fn `UserConstructionScript`)