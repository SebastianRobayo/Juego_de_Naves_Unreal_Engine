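; Curador is a moving healing pickup that restores health to the player's ship (Jugador_Nave).
; Each Tick moves it along local X by Velocidad without delta-time scaling or sweep, and a Delay of TiempoDeVida leads to its destruction.
; On overlap it adds Potenciadores to the ship's VidaJugador, then destroys itself whatever actor it touched.
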(event `self.ReceiveTick`
  (params (DeltaSeconds :type "Float (single-precision)"))
  ;[1 1 1] Movimiento del curador
  (`self.K2_AddActorLocalOffset` (`KismetMathLibrary.MakeVector` (`self.Velocidad`)))
  (`KismetSystemLibrary.Delay` (`self.Tiempo de vida`))
  (`self.K2_DestroyActor`))

(event `self.ReceiveActorBeginOverlap`
  (params (OtherActor :type "Actor Object Reference"))
  ;[1 1 1] Sistema de puntos
  (`|ExecutionSequence`
    (:`then_0`
      (bind _asjugador_nave (cast `/Game/Blueprint/Jugador_Nave/Jugador_Nave` OtherActor))
      (set `/Game/Blueprint/Jugador_Nave/Jugador_Nave.Vida_Jugador` (+ (`/Game/Blueprint/Jugador_Nave/Jugador_Nave.Vida_Jugador` _asjugador_nave) (`self.Potenciadores`)) _asjugador_nave))
    (:`then_1`
      (`self.K2_DestroyActor`))))

(fn `UserConstructionScript`)