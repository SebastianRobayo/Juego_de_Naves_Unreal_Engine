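; Game mode Blueprint that watches the score (Puntaje) and advances the game to Nivel2 when the player wins.
; A looping Delay started on BeginPlay periodically prints the current score to the screen.
; Tick checks the score every frame and, once it reaches the winning threshold, prints a victory message and opens the next level.
; Nothing in this file changes the score.
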(event `self.ReceiveBeginPlay`
  (`KismetSystemLibrary.Delay` 2.0 :!label _label)
  (`KismetSystemLibrary.PrintString` (`KismetStringLibrary.Conv_IntToString` (`self.Puntaje`)))
  (goto _label))

(event `self.ReceiveTick`
  (params (DeltaSeconds :type "Float (single-precision)"))
  (`|ExecutionSequence`
    (:`then_0`
      (if (>= (`self.Puntaje`) 10)
        (`KismetSystemLibrary.PrintString` "VICTORIA!!")
        (`GameplayStatics.OpenLevel` (`self.Nivel2`))))))

(fn `UserConstructionScript`)