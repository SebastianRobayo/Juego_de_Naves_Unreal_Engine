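; Player bullet actor for a ship shooter that damages Enemigo_Nave enemies and awards points.
; Tick moves it along local X by Velocidad per frame, unscaled by delta time and without sweep, while a Delay destroys it after VidaDeBala.
; On overlap it subtracts Daño from enemy health, increments Modo_de_Juego's Puntaje at zero or below, and destroys itself.
; Left mouse press and release play and stop the laser sound.
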(event `self.ReceiveTick`
  (params (DeltaSeconds :type "Float (single-precision)"))
  ;[1 1 1] Sistema de movimiento de la bala
  (`self.K2_AddActorLocalOffset` (`KismetMathLibrary.MakeVector` (`self.Velocidad`)))
  (`KismetSystemLibrary.Delay` (`self.Vida_de_Bala`))
  (`self.K2_DestroyActor`))

(event `Key|LeftMouseButton`
  (params (Key :type "Key Structure"))
  (bind _disparo_laser (`self.Disparo_Laser`))
  ;[1 1 1] Sonido de disparo
  (:`Pressed`
    (`AudioComponent.Play` _disparo_laser 0.0))
  (:`Released`
    (`AudioComponent.Stop` _disparo_laser)))

(event `self.ReceiveActorBeginOverlap`
  (params (OtherActor :type "Actor Object Reference"))
  ;[1 1 1] Sistema de destrucción del enemigo
  (`|ExecutionSequence`
    (:`then_0`
      (bind _asenemigo_nave (cast `/Game/Blueprint/Enemigo_Nave/Enemigo_Nave` OtherActor))
      (bind _vida_enemigo (`/Game/Blueprint/Enemigo_Nave/Enemigo_Nave.Vida_Enemigo` _asenemigo_nave))
      (set `/Game/Blueprint/Enemigo_Nave/Enemigo_Nave.Vida_Enemigo` (- _vida_enemigo (`self.Daño`)) _asenemigo_nave)
      (`self.K2_DestroyActor`))
    (:`then_1`
      (if (<= _vida_enemigo 0.0)
        (bind _asmodo_de_juego (cast `/Game/Blueprint/Modo_de_Juego/Modo_de_Juego` (`GameplayStatics.GetGameMode`)))
        (set `/Game/Blueprint/Modo_de_Juego/Modo_de_Juego.Puntaje` (+ (`/Game/Blueprint/Modo_de_Juego/Modo_de_Juego.Puntaje` _asmodo_de_juego) 1) _asmodo_de_juego)))
    (:`then_2`
      (`self.K2_DestroyActor`))))

(fn `UserConstructionScript`)