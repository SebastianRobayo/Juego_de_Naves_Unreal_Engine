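; Enemy ship that flies forward, fires bullets periodically and spawns a Curador (healer) when its health runs out.
; All logic runs from a Tick sequence, where a Delay throttles BalaDeEnemigo spawns at the actor's transform.
; Movement adds a local X offset of Velocidad each frame, without sweep or delta-time scaling.
; VidaEnemigo is polled every frame to trigger destruction and the Curador spawn; nothing here reduces it.
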(event `self.ReceiveTick`
  (params (DeltaSeconds :type "Float (single-precision)"))
  (`|ExecutionSequence`
    (:`then_0`
      ;[1 1 1] Sistema de disparo
      (`KismetSystemLibrary.Delay` (`self.Intervalo_Disparo`))
      (`|SpawnActorFromClass` (`self.Bala_de_Enemigo`) (`self.GetTransform`) "Undefined" "OverrideRootScale" null null))
    (:`then_1`
      ;[1 1 1] Sistema de movimiento
      (`self.K2_AddActorLocalOffset` (`KismetMathLibrary.MakeVector` (`self.Velocidad`))))
    (:`then_2`
      ;[1 1 1] Destrucción del enemigo y spawn de curadores
      (if (<= (`self.Vida_Enemigo`) 0.0)
        (`self.K2_DestroyActor`)
        (`|SpawnActorFromClass` "/Game/Blueprint/Curadores/Curador.Curador_C" (`self.GetTransform`) "Undefined" "OverrideRootScale" null null)))))

(fn `UserConstructionScript`)